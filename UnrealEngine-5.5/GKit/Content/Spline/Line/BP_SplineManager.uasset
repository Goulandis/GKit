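; BP_SplineManager is an actor for editing a mesh line through placed points on surfaces tagged VirtualShowroomFloor.
; Update takes a hit and, based on SplineManagerState, adds, deletes or selects BP_GPoint markers, which carry the same tag.
; UpdateLine moves the actor for the first point, otherwise rebuilds the spline and its runtime spline meshes from marker locations.
; Selection toggles a marker's position updating, highlights it, and rebuilds the line when updating stops.
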(fn `AddPoint`
  (params (Location :type "Vector Structure"))
  (bind _pointscale (`self.PointScale`))
  (bind _returnvalue (`|SpawnActorFromClass` "/GKit/Spline/Line/BP_GPoint.BP_GPoint_C" (`KismetMathLibrary.MakeTransform` (`KismetMathLibrary.MakeVector` Location_X Location_Y (+ Location_Z (`self.PointOffset`)))) "Undefined" "MultiplyWithRoot" null null))
  (`/GKit/Spline/Line/BP_GPoint.SetPointStyle` _returnvalue (`self.PointMesh`) (`KismetMathLibrary.MakeVector` _pointscale _pointscale _pointscale) (`self.PointMaterial`) false)
  (`KismetArrayLibrary.Array_AddUnique` (`Actor.Tags` _returnvalue) "VirtualShowroomFloor")
  (bind _returnvalue_2 (`KismetArrayLibrary.Array_AddUnique` (`self.Arr_Points`) _returnvalue))
  (set `self.Index` _returnvalue_2)
  (set `/GKit/Spline/Line/BP_GPoint.PointOffset` (`self.PointOffset`) _returnvalue))

(fn `ClearAll`
  (bind _spline (`self.Spline`))
  (bind _arr_splinemesh (`self.Arr_SplineMesh`))
  (for _array_element _arr_splinemesh
    (`ActorComponent.K2_DestroyComponent` _array_element))
  (`KismetArrayLibrary.Array_Clear` _arr_splinemesh)
  (for _array_element_2 (`self.Arr_Points`)
    (`self.K2_DestroyActor` _array_element_2)
    (while (> (`SplineComponent.GetNumberOfSplinePoints` _spline) 0)
      (`SplineComponent.RemoveSplinePoint` _spline 0 true))))

(fn `ClearSplinePoint`
  (bind _spline (`self.Spline`))
  (bind _arr_splinemesh (`self.Arr_SplineMesh`))
  (for _array_element _arr_splinemesh
    (`ActorComponent.K2_DestroyComponent` _array_element))
  (`KismetArrayLibrary.Array_Clear` _arr_splinemesh)
  (while (> (`SplineComponent.GetNumberOfSplinePoints` _spline) 0)
    (`SplineComponent.RemoveSplinePoint` _spline 0 true)))

(fn `DeletePoint`
  (params (Point :type "/GKit/Spline/Line/BP_GPoint Object Reference"))
  (if (>= (`KismetArrayLibrary.Array_Find` (`self.Arr_Points`) Point) 0)
    (`KismetArrayLibrary.Array_RemoveItem` (`self.Arr_Points`) Point)
    (`self.K2_DestroyActor` Point)))

(fn `SelectPoint`
  (params (Hit :type "HitResult Structure"))
  (bind _asbp_gpoint (cast `/GKit/Spline/Line/BP_GPoint` (`.HitActor` (`GameplayStatics.BreakHitResult` Hit))))
  (bind _output_get (set `self.CurrentSelectPoint` _asbp_gpoint))
  (set `/GKit/Spline/Line/BP_GPoint.StartUpdatePos` (not (`/GKit/Spline/Line/BP_GPoint.StartUpdatePos` _output_get)) _output_get)
  (`/GKit/Spline/Line/BP_GPoint.SetMaterial` _output_get (`self.PointSelectMaterial`))
  (for _array_element (`self.Arr_Points`)
    (if (!= _array_element (`self.CurrentSelectPoint`))
      (if (== (`PrimitiveComponent.GetMaterial` (`/GKit/Spline/Line/BP_GPoint.StaticMesh` _array_element) 0) (`self.PointSelectMaterial`))
        (`/GKit/Spline/Line/BP_GPoint.SetMaterial` _array_element (`self.PointMaterial`)))))
  (if (not (`/GKit/Spline/Line/BP_GPoint.StartUpdatePos` (`self.CurrentSelectPoint`)))
    (`self.UpdateLine` (struct))))

(fn `SetSplineType`
  (params (Comp :type "SplineMeshComponent Object Reference"))
  (bind _splinescale (`self.SplineScale`))
  (bind _returnvalue (`KismetMathLibrary.MakeVector2D` _splinescale _splinescale))
  (`SplineMeshComponent.SetStartScale` Comp _returnvalue true)
  (`SplineMeshComponent.SetEndScale` Comp _returnvalue true)
  (`StaticMeshComponent.SetStaticMesh` Comp (`self.SplineMesh`))
  (`PrimitiveComponent.SetMaterial` Comp 0 (`self.SplineMaterial`))
  (`PrimitiveComponent.SetCastShadow` Comp (`self.CastShadow`)))

(fn `Update`
  (params (Hit :type "HitResult Structure"))
  (bind _hit (`local.Hit`))
  (bind (_bblockinghit _binitialoverlap _time _distance _location _impactpoint _normal _impactnormal _physmat _hitactor) (`GameplayStatics.BreakHitResult` _hit))
  (if (`self.ActorHasTag` (`.HitActor` (`GameplayStatics.BreakHitResult` Hit)) "VirtualShowroomFloor")
    (switch `/GKit/Spline/Line/E_SplineManagerState` (`self.SplineManagerState`)
      (:`NewEnumerator1`
        (`self.AddPoint` _location)
        (`self.UpdateLine` _hit)
        (`self.UpdatePointState`))
      (:`NewEnumerator2`
        (bind _asbp_gpoint (cast `/GKit/Spline/Line/BP_GPoint` _hitactor))
        (`self.DeletePoint` _asbp_gpoint)
        (`self.UpdateLine` (`local.Hit`))
        (`self.UpdatePointState`))
      (:`NewEnumerator4`
        (`self.SelectPoint` _hit)))))

(fn `UpdateLine`
  (params (Hit :type "HitResult Structure"))
  (locals (HitLocation :type "Vector Structure"))
  (bind _spline (`self.Spline`))
  (set `local.HitLocation` (`.Location` (`GameplayStatics.BreakHitResult` Hit)))
  (if (== (`self.Index`) 0)
    (`self.K2_SetActorLocation` (`local.HitLocation`))
    (else
      (`self.ClearSplinePoint`)
      (for _array_element (`self.Arr_Points`)
        (`SplineComponent.AddSplinePoint` (`self.Spline`) (`self.K2_GetActorLocation` _array_element) "World" true)
        (for _index (range (`SplineComponent.GetNumberOfSplinePoints` (`self.Spline`)))
          (bind _returnvalue (`AddComponent|NODE_AddSplineMeshComponent-1` :`bManualAttachment` true))
          (`SceneComponent.SetMobility` _returnvalue "Movable")
          (`SceneComponent.K2_AttachToComponent` (`self.SplineMeshRoot`) _returnvalue "None" "KeepRelative" "KeepRelative" "KeepRelative" true)
          (`KismetArrayLibrary.Array_Add` (`self.Arr_SplineMesh`) _returnvalue)
          (`self.SetSplineType` _returnvalue)
          (bind (_location _tangent) (`SplineComponent.GetLocationAndTangentAtSplinePoint` _spline (- _index 1) "World"))
          (bind (_location_2 _tangent_2) (`SplineComponent.GetLocationAndTangentAtSplinePoint` _spline _index "World"))
          (`SplineMeshComponent.SetStartAndEnd` _returnvalue _location _tangent _location_2 _tangent_2 true))))))

(fn `UpdatePointState`
  (for _array_element (`self.Arr_Points`)
    (if (== (`PrimitiveComponent.GetMaterial` (`/GKit/Spline/Line/BP_GPoint.StaticMesh` _array_element) 0) (`self.PointSelectMaterial`))
      (`/GKit/Spline/Line/BP_GPoint.SetMaterial` _array_element (`self.PointMaterial`))))
  (set `self.CurrentSelectPoint` null))

(fn `UserConstructionScript`)