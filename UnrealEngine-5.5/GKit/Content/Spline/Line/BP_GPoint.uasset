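; BP_GPoint is a point marker actor, apparently for the spline line tool, that can be dragged across the virtual showroom floor.
; While StartUpdatePos is set, Tick traces from the deprojected mouse cursor on the Visibility channel.
; Hits on actors tagged VirtualShowroomFloor move the point there, raised by PointOffset.
; Helper functions set its mesh, scale, material and shadow casting, or swap the material alone.
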(event `self.ReceiveTick`
  (params (DeltaSeconds :type "Float (single-precision)"))
  (bind (_worldlocation _worlddirection) (`PlayerController.DeprojectMousePositionToWorld` (`GameplayStatics.GetPlayerController` 0)))
  (if (`self.StartUpdatePos`)
    (bind _outhit (`KismetSystemLibrary.LineTraceSingle` _worldlocation (+ (* _worlddirection 10000000.0) _worldlocation) "TraceTypeQuery1"))
    (bind (_bblockinghit _binitialoverlap _time _distance _location _impactpoint _normal _impactnormal _physmat _hitactor) (`GameplayStatics.BreakHitResult` _outhit))
    (if (`self.ActorHasTag` _hitactor "VirtualShowroomFloor")
      (`self.K2_SetActorLocation` (`KismetMathLibrary.MakeVector` (.x _location) (.y _location) (+ (.z _location) (`self.PointOffset`)))))))

(fn `SetMaterial`
  (params (Mat :type "MaterialInstance Object Reference"))
  (`PrimitiveComponent.SetMaterial` (`self.StaticMesh`) 0 Mat))

(fn `SetPointStyle`
  (params (Mesh :type "StaticMesh Object Reference") (Scale :type "Vector Structure" :default (1.0 1.0 1.0)) (Material :type "MaterialInstance Object Reference") (CastShadow :type Boolean))
  (bind _staticmesh (`self.StaticMesh`))
  (`StaticMeshComponent.SetStaticMesh` _staticmesh Mesh)
  (`SceneComponent.SetWorldScale3D` _staticmesh Scale)
  (`PrimitiveComponent.SetMaterial` _staticmesh 0 Material)
  (`PrimitiveComponent.SetCastShadow` _staticmesh CastShadow))

(fn `UserConstructionScript`)