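; Spline line manager that builds an editable line from BP_GPoint actors placed, deleted or selected via hits on ClickPlane-tagged actors.
; UpdateByHit branches on the manager state to spawn, destroy or toggle position updating on a point, highlighting the selection by material.
; UpdateLine clears and rebuilds the spline from point locations, creating spline mesh components styled with shared mesh, scale, material and shadow settings.
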(fn `AddPoint`
  (params (Location :type "Vector Structure"))
  (bind _pointscale (`self.PointScale`))
  (bind _returnvalue (`|SpawnActorFromClass` "/GKit/Development/Spline/Line/BP_GPoint.BP_GPoint_C" (`KismetMathLibrary.MakeTransform` (`KismetMathLibrary.MakeVector` Location_X Location_Y (+ Location_Z (`self.PointOffset`)))) "Undefined" "MultiplyWithRoot" null null))
  (`/GKit/Development/Spline/Line/BP_GPoint.SetPointStyle` _returnvalue (`self.PointMesh`) (`KismetMathLibrary.MakeVector` _pointscale _pointscale _pointscale) (`self.PointMaterial`) (`self.CastShadow`))
  (`KismetArrayLibrary.Array_AddUnique` (`Actor.Tags` _returnvalue) "VirtualShowroomFloor")
  (bind _returnvalue_2 (`KismetArrayLibrary.Array_AddUnique` (`self.Arr_Points`) _returnvalue))
  (set `self.Index` _returnvalue_2)
  (set `/GKit/Development/Spline/Line/BP_GPoint.PointOffset` (`self.PointOffset`) _returnvalue))

(fn `ClearAll`
  (bind _spline (`self.Spline`))
  (bind _arr_points (`self.Arr_Points`))
  (bind _arr_splinemesh (`self.Arr_SplineMesh`))
  (`ActorComponent.K2_DestroyComponent` _arr_splinemesh)
  (`KismetArrayLibrary.Array_Clear` _arr_splinemesh)
  (for _array_element _arr_points
    (`self.K2_DestroyActor` _array_element)
    (while (> (`SplineComponent.GetNumberOfSplinePoints` _spline) 0)
      (`SplineComponent.RemoveSplinePoint` _spline 0 true)))
  (`KismetArrayLibrary.Array_Clear` _arr_points))

(fn `ClearSplinePoint`
  (bind _spline (`self.Spline`))
  (bind _arr_splinemesh (`self.Arr_SplineMesh`))
  (`ActorComponent.K2_DestroyComponent` _arr_splinemesh)
  (`KismetArrayLibrary.Array_Clear` _arr_splinemesh)
  (while (> (`SplineComponent.GetNumberOfSplinePoints` _spline) 0)
    (`SplineComponent.RemoveSplinePoint` _spline 0 true)))

(fn `DeletePoint`
  (params (Point :type "/GKit/Development/Spline/Line/BP_GPoint Object Reference"))
  (if (`KismetArrayLibrary.Array_Contains` (`self.Arr_Points`) Point)
    (`KismetArrayLibrary.Array_RemoveItem` (`self.Arr_Points`) Point)
    (`self.K2_DestroyActor` Point)))

(fn `FindPointByPos`
  (params (Pos :type "Vector Structure"))
  (returns (Point :type "/GKit/Development/Spline/Line/BP_GPoint Object Reference"))
  (for _array_element (`self.Arr_Points`)
    (if (== (`self.K2_GetActorLocation` _array_element) Pos :`ErrorTolerance` 1.0)
      (return _array_element)))
  (return null))

(fn `SelectPoint`
  (params (Hit :type "HitResult Structure"))
  (bind _asbp_gpoint (cast `/GKit/Development/Spline/Line/BP_GPoint` (`.HitActor` (`GameplayStatics.BreakHitResult` Hit))))
  (bind _output_get (set `self.CurrentSelectPoint` _asbp_gpoint))
  (set `/GKit/Development/Spline/Line/BP_GPoint.StartUpdatePos` (not (`/GKit/Development/Spline/Line/BP_GPoint.StartUpdatePos` _output_get)) _output_get)
  (`/GKit/Development/Spline/Line/BP_GPoint.SetMaterial` _output_get (`self.PointSelectMaterial`))
  (for _array_element (`self.Arr_Points`)
    (if (!= _array_element (`self.CurrentSelectPoint`))
      (if (== (`PrimitiveComponent.GetMaterial` (`/GKit/Development/Spline/Line/BP_GPoint.StaticMesh` _array_element) 0) (`self.PointSelectMaterial`))
        (`/GKit/Development/Spline/Line/BP_GPoint.SetMaterial` _array_element (`self.PointMaterial`)))))
  (if (not (`/GKit/Development/Spline/Line/BP_GPoint.StartUpdatePos` (`self.CurrentSelectPoint`)))
    (`self.UpdateLine`)))

(fn `SetSplineType`
  (params (Comp :type "SplineMeshComponent Object Reference"))
  (bind _splinescale (`self.SplineScale`))
  (bind _returnvalue (`KismetMathLibrary.MakeVector2D` _splinescale _splinescale))
  (`SplineMeshComponent.SetStartScale` Comp _returnvalue true)
  (`SplineMeshComponent.SetEndScale` Comp _returnvalue true)
  (`StaticMeshComponent.SetStaticMesh` Comp (`self.SplineMesh`))
  (`PrimitiveComponent.SetMaterial` Comp 0 (`self.SplineMaterial`))
  (`PrimitiveComponent.SetCastShadow` Comp (`self.CastShadow`)))

(fn `UpdateByHit`
  (params (Hit :type "HitResult Structure"))
  (bind _hit (`local.Hit`))
  (bind (_bblockinghit _binitialoverlap _time _distance _location _impactpoint _normal _impactnormal _physmat _hitactor) (`GameplayStatics.BreakHitResult` _hit))
  (if (`self.ActorHasTag` (`.HitActor` (`GameplayStatics.BreakHitResult` Hit)) "ClickPlane")
    (switch `/GKit/Development/Spline/Line/E_SplineManagerState` (`self.SplineManagerState`)
      (:`NewEnumerator1`
        (`self.AddPoint` _location)
        (`self.UpdateLine`)
        (`self.UpdatePointState`))
      (:`NewEnumerator2`
        (bind _asbp_gpoint (cast `/GKit/Development/Spline/Line/BP_GPoint` _hitactor))
        (`self.DeletePoint` _asbp_gpoint)
        (`self.UpdateLine`)
        (`self.UpdatePointState`))
      (:`NewEnumerator3`
        (`self.SelectPoint` _hit)))))

(fn `UpdateLine`
  (locals (HitLocation :type "Vector Structure"))
  (bind _arr_points (`self.Arr_Points`))
  (bind _spline (`self.Spline`))
  (`self.ClearSplinePoint`)
  (for _index (range (+ (`KismetArrayLibrary.Array_LastIndex` _arr_points) 1))
    (`SplineComponent.AddSplinePointAtIndex` (`self.Spline`) (`self.K2_GetActorLocation` (`|GetArrayItem` _arr_points _index)) _index "World" true)
    (bind _returnvalue (`AddComponent|NODE_AddSplineMeshComponent-1` :`bManualAttachment` true))
    (`SceneComponent.SetMobility` _returnvalue "Movable")
    (`SceneComponent.K2_AttachToComponent` (`self.SplineMeshRoot`) _returnvalue "None" "KeepRelative" "KeepRelative" "KeepRelative" true)
    (`KismetArrayLibrary.Array_Add` (`self.Arr_SplineMesh`) _returnvalue)
    (`self.SetSplineType` _returnvalue)
    (if (> _index 0)
      (bind (_location _tangent) (`SplineComponent.GetLocationAndTangentAtSplinePoint` _spline (- _index 1) "World"))
      (bind (_location_2 _tangent_2) (`SplineComponent.GetLocationAndTangentAtSplinePoint` _spline _index "World"))
      (`SplineMeshComponent.SetStartAndEnd` _returnvalue _location _tangent _location_2 _tangent_2 true))))

(fn `UpdatePointState`
  (for _array_element (`self.Arr_Points`)
    (if (== (`PrimitiveComponent.GetMaterial` (`/GKit/Development/Spline/Line/BP_GPoint.StaticMesh` _array_element) 0) (`self.PointSelectMaterial`))
      (`/GKit/Development/Spline/Line/BP_GPoint.SetMaterial` _array_element (`self.PointMaterial`))))
  (set `self.CurrentSelectPoint` null))

(fn `UserConstructionScript`)